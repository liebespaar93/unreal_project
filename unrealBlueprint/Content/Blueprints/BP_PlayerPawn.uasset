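; Player-controlled shooter pawn that moves on the XY plane and fires BP_Bullet.
; BeginPlay adds the IMC_MyInput Enhanced Input context, whose actions store horizontal and vertical values and fire bullets from FirePosition with a laser sound.
; Tick normalizes the input vector and moves the pawn by speed and delta time through SetActorLocation without sweeping.
; Legacy axis events and their disconnected nodes remain unused.
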(event Input|EnhancedActionEvents|EnhancedInputActionIA_Horizontal
  (params (ActionValue :type Float%20%28double-precision%29) (ElapsedSeconds :type Float%20%28double-precision%29) (TriggeredSeconds :type Float%20%28double-precision%29) (InputAction :type Input%20Action%20Object%20Reference :default "/Game/EnhanceInput/IA_Horizontal.IA_Horizontal"))
  ;[1 1 1] Comment
  ;;[1 1 1] Comment
  (:Triggered
    (Variables|Default|SetHorizontal ActionValue))
  (:Completed
    (Variables|Default|SetHorizontal ActionValue)))

(event Input|EnhancedActionEvents|EnhancedInputActionIA_Vertical
  (params (ActionValue :type Float%20%28double-precision%29) (ElapsedSeconds :type Float%20%28double-precision%29) (TriggeredSeconds :type Float%20%28double-precision%29) (InputAction :type Input%20Action%20Object%20Reference :default "/Game/EnhanceInput/IA_Vertical.IA_Vertical"))
  ;[1 1 1] Comment
  ;;[1 1 1] Comment
  (:Triggered
    (Variables|Default|SetVertical ActionValue))
  (:Completed
    (Variables|Default|SetVertical ActionValue)))

(event Input|EnhancedActionEvents|EnhancedInputActionIA_Fire
  (params (ActionValue :type Boolean) (ElapsedSeconds :type Float%20%28double-precision%29) (TriggeredSeconds :type Float%20%28double-precision%29) (InputAction :type Input%20Action%20Object%20Reference :default "/Game/EnhanceInput/IA_Fire.IA_Fire"))
  (bind _fireposition (Variables|Default|GetFirePosition))
  ;[1 1 1] Comment
  ;;[1 1 1] Comment
  (Game|SpawnActorfromClass "/Game/Blueprints/BP_Bullet.BP_Bullet_C" (Math|Transform|MakeTransform (Transformation|GetWorldLocation _fireposition) (Transformation|GetWorldRotation _fireposition) "1.000000,1.000000,1.000000") "Undefined" "MultiplyWithRoot" 0 0)
  (Audio|PlaySound2D "/Game/Sounds/one-shote-laser.one-shote-laser" 1.0 1.0 0.0 0 0))

(event EventBeginPlay
  ;[1 1 1] Setting Input Mapping
  (Input|AddMappingContext (PlayerController|LocalPlayerSubsystems|GetEnhancedInputLocalPlayerSubsystem (Game|GetPlayerController 0)) "/Game/EnhanceInput/IMC_MyInput.IMC_MyInput" 0 "(bIgnoreAllPressedKeysUntilRelease=True,bForceImmediately=False,bNotifyUserSettings=False)"))

(event EventTick
  (params (DeltaSeconds :type Float%20%28single-precision%29))
  ;[1 1 1] movement funtion (P = P0 + vt)
  (bind _output_get (Variables|Default|SetDirection (Math|Vector|MakeVector (Variables|Default|GetVertical) (Variables|Default|GetHorizontal) 0.0)))
  (Transformation|SetActorLocation (+ (* (* (Math|Vector|Normalize _output_get) (Variables|Default|GetMovespeed)) DeltaSeconds) (Transformation|GetActorLocation)) false false))

(event Collision|EventActorBeginOverlap
  (params (OtherActor :type Actor%20Object%20Reference)))

(event Input|ActionEvents|InputActionFire
  (params (Key :type Key%20Structure :default "None"))
  ;[1 1 1] fire bullet
)

(event Input|AxisEvents|InputAxisHorizontal
  (params (AxisValue :type Float%20%28single-precision%29))
  ;[1 1 1] movement funtion (P = P0 + vt)
)

(event Input|AxisEvents|InputAxisVertical
  (params (AxisValue :type Float%20%28single-precision%29))
  ;[1 1 1] movement funtion (P = P0 + vt)
)

(fn ConstructionScript)