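; BP_EnemyFactory is an actor that repeatedly spawns BP_Enemy actors at a fixed interval.
; Each Tick adds delta time to CurrentTime until it reaches SpawnTime.
; It then spawns an enemy at the EnemyPosition component's world location and rotation and resets the timer to zero.
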(event EventBeginPlay)

(event Collision|EventActorBeginOverlap
  (params (OtherActor :type Actor%20Object%20Reference)))

(event EventTick
  (params (DeltaSeconds :type Float%20%28single-precision%29))
  (bind _enemyposition (Variables|Default|GetEnemyPosition))
  ;[1 1 1] Check Maximum CurrentTime
  (bind _output_get (Variables|Default|SetCurrentTime (+ DeltaSeconds (Variables|Default|GetCurrentTime))))
  (if (>= _output_get (Variables|Default|GetSpawnTime))
    ;[1 1 1] Spawn Enemy
    (Game|SpawnActorfromClass "/Game/Blueprints/BP_Enemy.BP_Enemy_C" (Math|Transform|MakeTransform (Transformation|GetWorldLocation _enemyposition) (Transformation|GetWorldRotation _enemyposition) "1.000000,1.000000,1.000000") "Undefined" "MultiplyWithRoot" 0 0)
    (Variables|Default|SetCurrentTime 0.0)))

(fn ConstructionScript)