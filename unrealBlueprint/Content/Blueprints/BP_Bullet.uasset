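; BP_Bullet is a projectile actor that flies straight and destroys enemies it hits.
; On BeginPlay it stores its forward vector, then each Tick moves along that direction at Movespeed scaled by delta time, without sweeping.
; When its Box component overlaps a BP_Enemy, it spawns an explosion effect at the enemy, plays a 2D sound, and destroys both the enemy and itself.
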(event OnComponentBeginOverlap(Box)
  (params (OverlappedComponent :type Primitive%20Component%20Object%20Reference) (OtherActor :type Actor%20Object%20Reference) (OtherComp :type Primitive%20Component%20Object%20Reference) (OtherBodyIndex :type Integer) (bFromSweep :type Boolean) (SweepResult :type Hit%20Result%20Structure%20%28by%20ref%29))
  ;[1 1 1] Bullet Destroy Enemy
  (bind _asbp_enemy (Utilities|Casting|CastToBP_Enemy OtherActor))
  (Effects|SpawnEmitteratLocation "/Game/StarterContent/Particles/P_Explosion.P_Explosion" (Transformation|GetActorLocation _asbp_enemy))
  (Audio|PlaySound2D "/Game/StarterContent/Audio/Explosion01.Explosion01" 1.0 1.0 0.0 0 0)
  (Actor|DestroyActor _asbp_enemy)
  (Actor|DestroyActor))

(event EventBeginPlay
  ;[1 1 1] Direction Set
  (Variables|Default|SetDirection (Transformation|GetActorForwardVector)))

(event Collision|EventActorBeginOverlap
  (params (OtherActor :type Actor%20Object%20Reference)))

(event EventTick
  (params (DeltaSeconds :type Float%20%28single-precision%29))
  ;[1 1 1] Bullet movement
  (Transformation|SetActorLocation (+ (* (* (Math|Vector|Normalize (Variables|Default|GetDirection)) (Variables|Default|GetMovespeed)) DeltaSeconds) (Transformation|GetActorLocation)) false false))

(fn ConstructionScript)