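; BP_FirstBlueprint is a practice Blueprint for basic scripting, with no gameplay behavior beyond printing to screen.
; On BeginPlay it passes two number variables to its Add function and prints the sum.
; Separate Branch and NewFunction functions demonstrate a boolean check and a counting loop, but nothing in the file calls them.
; Tick, overlap and the construction script are empty.
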(event EventBeginPlay
  (bind _result (CallFunction|Add (Variables|Default|GetNumber1) (Variables|Default|GetNumber2)))
  (Development|PrintString (Utilities|String|ToString(Integer) _result)))

(event Collision|EventActorBeginOverlap
  (params (OtherActor :type Actor%20Object%20Reference)))

(event EventTick
  (params (DeltaSeconds :type Float%20%28single-precision%29)))

(fn ConstructionScript)

(fn Add
  (params (number1 :type Integer) (number2 :type Integer))
  (return (+ number1 number2)))

(fn Branch
  (if (Variables|Default|GetisMan)
    (Development|PrintString "man real?")
    (else
      (Development|PrintString "not man real?"))))

(fn NewFunction
  (for _index (range 0 9)
    (Development|PrintString (Utilities|String|ToString(Integer) _index))))