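; Base AI character Blueprint that provides chase, fire and gun-equip actions.
; ChasePlayer uses AIMoveTo toward player 0, re-issuing it after a short delay only on success.
; EquippingGun, marked temporary, spawns a BP_KA47, attaches it to the hand socket, plays a pull-out montage, then sets EquipGun.
; Fire only plays a montage; both gun actions call end dispatchers whether their montage completes or is interrupted.
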(event Custom|ChasePlayer
  ;[1 1 1] 따라다니기
  (AI|AIMoveTo self "0, 0, 0" (Game|GetPlayerCharacter 0) 5.0 false
    (:OnSuccess
      (Utilities|FlowControl|Delay 0.2)
      (CallFunction|ChasePlayer))))

(event Custom|Fire
  ;[1 1 1] 총쏘기
  (Animation|Montage|PlayMontage (Variables|Character|GetMesh) "/Game/Kyoulee/AICharacter/Motages/FiringRifle_UE_Montage.FiringRifle_UE_Montage"
    (:OnCompleted
      _)
    (:OnInterrupted
      _))
  (Default|CallOnFireEnd))

(event Custom|EquippingGun
  ;[1 1 1] 장착하기 (임시)
  (bind _returnvalue (Game|SpawnActorfromClass "/Game/Kyoulee/AICharacter/BP_KA47.BP_KA47_C" (Transformation|GetActorTransform) "AlwaysSpawn" "MultiplyWithRoot" 0 0))
  (bind _output_get (Variables|Default|SetWeapon _returnvalue))
  (Transformation|AttachComponentToComponent _output_get (Variables|Character|GetMesh) "hand_rSocket" "SnapToTarget" "SnapToTarget" "SnapToTarget" true)
  (Animation|Montage|PlayMontage (Variables|Character|GetMesh) "/Game/Kyoulee/AICharacter/Motages/RiflePullOut_UE_Montage.RiflePullOut_UE_Montage"
    (:OnCompleted
      _)
    (:OnInterrupted
      _))
  (Variables|Default|SetEquipGun true)
  (Default|CallOnEquipGunEnd))

(event EventBeginPlay)

(event Collision|EventActorBeginOverlap
  (params (OtherActor :type Actor%20Object%20Reference)))

(event EventTick
  (params (DeltaSeconds :type Float%20%28single-precision%29)))

(fn ConstructionScript)