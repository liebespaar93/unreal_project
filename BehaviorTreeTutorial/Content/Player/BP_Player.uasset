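; BP_Player is the player Blueprint, with keyboard controls that switch the state of an AI character.
; On BeginPlay it enables input from player controller 0.
; Keys 1 and 2 look up a BP_AICharacter_Base with GetActorOfClass and cast its controller to AIC_AICharacter_Base.
; Key 1 sets that controller to the attack state with the player as target, and key 2 returns it to idle.
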(event EventBeginPlay
  (Input|EnableInput self (Game|GetPlayerController 0)))

(event Collision|EventActorBeginOverlap
  (params (OtherActor :type Actor%20Object%20Reference)))

(event EventTick
  (params (DeltaSeconds :type Float%20%28single-precision%29)))

(event Input|KeyboardEvents|1
  (params (Key :type Key%20Structure :default "None"))
  (:Pressed
    (bind _returnvalue (Actor|GetActorOfClass "/Game/Kyoulee/AICharacter/BP_AICharacter_Base.BP_AICharacter_Base_C"))
    (bind _asaic_aicharacter_base (Utilities|Casting|CastToAIC_AICharacter_Base (AI|GetAIController _returnvalue)))
    (Default|SetAiStateAttack _asaic_aicharacter_base self)))

(event Input|KeyboardEvents|2
  (params (Key :type Key%20Structure :default "None"))
  (:Pressed
    (bind _returnvalue (Actor|GetActorOfClass "/Game/Kyoulee/AICharacter/BP_AICharacter_Base.BP_AICharacter_Base_C"))
    (bind _asaic_aicharacter_base (Utilities|Casting|CastToAIC_AICharacter_Base (AI|GetAIController _returnvalue)))
    (Default|SetAiStateIdle _asaic_aicharacter_base)))

(fn ConstructionScript)